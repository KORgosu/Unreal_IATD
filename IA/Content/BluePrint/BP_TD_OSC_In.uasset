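; BP_TD_OSC_In is an OSC receiver that lets incoming network messages control the BPOverheadLight actors in the level.
; On BeginPlay it starts a listening OSC server on a configurable address and port, gathers those lights and randomizes their color.
; Its message handler matches the "/intensity" address and passes the first float to SetIntensity on the lights gathered at BeginPlay.
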(event Custom|OnMsgReceived
  (params (Message :type OSC%20Message%20Structure%20%28by%20ref%29) (IPAddress :type String) (Port :type Integer))
  ;[1 1 1] Binding to Any Message
  (bind _returnvalue (Class|OSCManager|GetOSCMessageAddress Message))
  (bind _returnvalue_2 (Class|OSCManager|GetOSCAddressFullPath _returnvalue))
  (if (Class|KismetStringLibrary|MatchesWildcard _returnvalue_2 "/intensity" "IgnoreCase")
    (bind _value (Class|OSCManager|GetFloat Message))
    (Default|SetIntensity (stale EventBeginPlay _outactors) _value)))

(event EventBeginPlay
  ;[1 1 1] Binding to Any Message
  (bind _returnvalue (Class|OSCManager|CreateOSCServer (Variables|Default|GetReceive%20IPAddress) (Variables|Default|GetPort) false true "UE_OSC" 0))
  (bind _output_get (Variables|Default|SetTD_OSC_Server _returnvalue))
  (EventDispatchers|AssignOnOscMessageReceived _output_get (delegate Custom|OnMsgReceived))
  (bind _outactors (Actor|GetAllActorsOfClass (Variables|Default|GetBP_Overhead_Light)))
  (Default|SetRandomColor _outactors))

(event Collision|EventActorBeginOverlap
  (params (OtherActor :type Actor%20Object%20Reference)))

(event EventTick
  (params (DeltaSeconds :type Float%20%28single-precision%29)))

(fn ConstructionScript)